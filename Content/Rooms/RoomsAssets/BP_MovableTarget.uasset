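; BP_MovableTarget is a shooting target that slides side to side in a room until a projectile hits it.
; Tick moves it along relative Y at a random speed and starting direction, reversing on Box overlaps with anything except other movable targets.
; A BP_Projectile hit stops movement and plays a timeline tipping it 90 degrees in pitch.
; It then destroys itself and calls TargetShoot on its F1R3 or F3R2 parent actor.
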(event OnComponentHit(Target1)
  (params (HitComponent :type Primitive%20Component%20Object%20Reference) (OtherActor :type Actor%20Object%20Reference) (OtherComp :type Primitive%20Component%20Object%20Reference) (NormalImpulse :type Vector :default "0, 0, 0") (Hit :type Hit%20Result%20Structure%20%28by%20ref%29))
  (bind _returnvalue (Actor|GetParentActor))
  (bind _target (Variables|Default|GetTarget))
  (bind _returnvalue_2 (Transformation|GetRelativeTransform _target))
  (Variables|Default|SetdownPos (Math|Transform|MakeTransform (.location _returnvalue_2) (Math|Rotator|MakeRotator (.roll (.rotation _returnvalue_2)) (+ (.pitch (.rotation _returnvalue_2)) 9e+01) (.yaw (.rotation _returnvalue_2))) (.scale _returnvalue_2)))
  (Utilities|Casting|CastToBP_Projectile OtherActor)
  (Variables|Default|SetMoving false)
  (bind _newtrack_0 (Timeline|Timeline_0 Play)
    (:Update
      (Transformation|SetRelativeTransform (Variables|Default|GetTarget) (Math|Transform|Lerp(Transform) (Transformation|GetRelativeTransform (Variables|Default|GetTarget)) (Variables|Default|GetdownPos) _newtrack_0) true false))
    (:Finished
      (Actor|DestroyActor)
      (bind _asf1r3 (Utilities|Casting|CastToF1R3 _returnvalue)
        (:then
          (Default|TargetShoot _asf1r3))
        (:CastFailed
          (bind _asf3r2 (Utilities|Casting|CastToF3R2 _returnvalue))
          (Default|TargetShoot _asf3r2))))))

(event OnComponentBeginOverlap(Box)
  (params (OverlappedComponent :type Primitive%20Component%20Object%20Reference) (OtherActor :type Actor%20Object%20Reference) (OtherComp :type Primitive%20Component%20Object%20Reference) (OtherBodyIndex :type Integer) (bFromSweep :type Boolean) (SweepResult :type Hit%20Result%20Structure%20%28by%20ref%29))
  (Utilities|Casting|CastToBP_MovableTarget OtherActor
    (:CastFailed
      (CallFunction|DirectionChenge))))

(event Custom|Direction%20chenge
  (if (Variables|Default|GetLeftMotion)
    (Variables|Default|SetLeftMotion false)
    (else
      (Variables|Default|SetLeftMotion true))))

(event EventBeginPlay
  (bind _target (Variables|Default|GetTarget))
  (bind _returnvalue (Transformation|GetRelativeTransform _target))
  (Variables|Default|SetdownPos (Math|Transform|MakeTransform (.location _returnvalue) (Math|Rotator|MakeRotator (.roll (.rotation _returnvalue)) (+ (.pitch (.rotation _returnvalue)) 9e+01) (.yaw (.rotation _returnvalue))) (.scale _returnvalue)))
  (Variables|Default|SetLeftMotion (Math|Random|RandomBool))
  (Variables|Default|SetSpeed (Math|Random|RandomFloatinRange (Variables|Default|GetSpeedMin) (Variables|Default|GetSpeedMax))))

(event EventTick
  (params (DeltaSeconds :type Float%20%28single-precision%29))
  (bind _target (Variables|Default|GetTarget))
  (bind _target_2 (Variables|Default|GetTarget))
  (bind _returnvalue (Transformation|GetRelativeTransform _target))
  (if (Variables|Default|GetMoving)
    (Variables|Default|SetDelta%20Seconds DeltaSeconds)
    (if (Variables|Default|GetLeftMotion)
      (Transformation|SetRelativeTransform _target_2 (Math|Transform|MakeTransform (Math|Vector|MakeVector (.x (.location _returnvalue)) (- (.y (.location _returnvalue)) (* (Variables|Default|GetSpeed) (Variables|Default|GetDelta%20Seconds))) (.z (.location _returnvalue))) (.rotation _returnvalue) (.scale _returnvalue)) true false)
      (else
        (Transformation|SetRelativeTransform _target_2 (Math|Transform|MakeTransform (Math|Vector|MakeVector (.x (.location _returnvalue)) (+ (.y (.location _returnvalue)) (* (Variables|Default|GetSpeed) (Variables|Default|GetDelta%20Seconds))) (.z (.location _returnvalue))) (.rotation _returnvalue) (.scale _returnvalue)) true false)))))

(fn ConstructionScript
  (Variables|Default|SetMoving true))