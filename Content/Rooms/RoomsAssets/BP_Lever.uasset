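; BP_Lever is an interactive room lever that opens a door in the room actor that owns it.
; Its Box overlap enables input only while the player character is inside, and pressing E alternates the lever's rotation and IsActive state.
; Only activation calls OpenDoor, which tries a cast chain on the parent actor across five specific room classes (F1R8, F2R4, F2R5, F3R5, F3R1) to trigger that room's door function.
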(event OnComponentBeginOverlap(Box)
  (params (OverlappedComponent :type Primitive%20Component%20Object%20Reference) (OtherActor :type Actor%20Object%20Reference) (OtherComp :type Primitive%20Component%20Object%20Reference) (OtherBodyIndex :type Integer) (bFromSweep :type Boolean) (SweepResult :type Hit%20Result%20Structure%20%28by%20ref%29))
  (Utilities|Casting|CastToBP_PlayerCharacter OtherActor)
  (Input|EnableInput (Game|GetPlayerController 0)))

(event OnComponentEndOverlap(Box)
  (params (OverlappedComponent :type Primitive%20Component%20Object%20Reference) (OtherActor :type Actor%20Object%20Reference) (OtherComp :type Primitive%20Component%20Object%20Reference) (OtherBodyIndex :type Integer))
  (Utilities|Casting|CastToBP_PlayerCharacter OtherActor)
  (Input|DisableInput (Game|GetPlayerController 0)))

(event Custom|Open%20Door
  (bind _returnvalue (Actor|GetParentActor))
  ;[1 1 1] Pokój F1R8 otwieranie drzwi.
  (bind _asf1r8 (Utilities|Casting|CastToF1R8 _returnvalue)
    (:then
      (Default|OpenDor _asf1r8))
    (:CastFailed
      ;[1 1 1] Pokój F2R4 otwieranie drzwi.
      (bind _asf2r4 (Utilities|Casting|CastToF2R4 _returnvalue)
        (:then
          (Default|OpenDor _asf2r4))
        (:CastFailed
          ;[1 1 1] Pokój F2R5 otwieranie drzwi
          (bind _asf2r5 (Utilities|Casting|CastToF2R5 _returnvalue)
            (:then
              (Default|OpenDor _asf2r5))
            (:CastFailed
              ;[1 1 1] Pokój F3R5 otwieranie drzwi
              (bind _asf3r5 (Utilities|Casting|CastToF3R5 _returnvalue)
                (:then
                  (Default|OpenDor _asf3r5))
                (:CastFailed
                  ;[1 1 1] Pokój F3R5 otwieranie drzwi
                  (bind _asf3r1 (Utilities|Casting|CastToF3R1 _returnvalue))
                  (Default|Opendoor _asf3r1))))))))))

(event Input|KeyboardEvents|E
  (params (Key :type Key%20Structure :default "None"))
  (:Pressed
    (Utilities|FlowControl|FlipFlop
      (:A
        (Variables|Default|SetisActive? true)
        (Transformation|AddRelativeRotation (Variables|Default|GetLever) "180.000000, 0, 0" false false)
        (CallFunction|OpenDoor))
      (:B
        (Variables|Default|SetisActive? false)
        (Transformation|AddRelativeRotation (Variables|Default|GetLever) "-180.000000, 0, 0" false false)))))

(fn ConstructionScript)