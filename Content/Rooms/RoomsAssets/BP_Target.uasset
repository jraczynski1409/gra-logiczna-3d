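; BP_Target is a shootable target that falls over when hit and reports to its F1R3 parent actor.
; At BeginPlay it stores a down pose with 90 degrees added pitch.
; A BP_Projectile hit on Target1 plays a timeline that lerps Target from its current transform toward that pose with sweep.
; When the timeline finishes, it destroys itself, then calls TargetShoot on the parent F1R3.
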(event OnComponentHit(Target1)
  (params (HitComponent :type Primitive%20Component%20Object%20Reference) (OtherActor :type Actor%20Object%20Reference) (OtherComp :type Primitive%20Component%20Object%20Reference) (NormalImpulse :type Vector :default "0, 0, 0") (Hit :type Hit%20Result%20Structure%20%28by%20ref%29))
  (Utilities|Casting|CastToBP_Projectile OtherActor)
  (bind _newtrack_0 (Timeline|Timeline_0 Play)
    (:Update
      (Transformation|SetRelativeTransform (Variables|Default|GetTarget) (Math|Transform|Lerp(Transform) (Transformation|GetRelativeTransform (Variables|Default|GetTarget)) (Variables|Default|GetdownPos) _newtrack_0) true false))
    (:Finished
      (Actor|DestroyActor)
      (bind _asf1r3 (Utilities|Casting|CastToF1R3 (Actor|GetParentActor)))
      (Default|TargetShoot _asf1r3))))

(event EventBeginPlay
  (bind _target (Variables|Default|GetTarget))
  (bind _returnvalue (Transformation|GetRelativeTransform _target))
  (Variables|Default|SetdownPos (Math|Transform|MakeTransform (.location _returnvalue) (Math|Rotator|MakeRotator (.roll (.rotation _returnvalue)) (+ (.pitch (.rotation _returnvalue)) 9e+01) (.yaw (.rotation _returnvalue))) (.scale _returnvalue))))

(event Collision|EventActorBeginOverlap
  (params (OtherActor :type Actor%20Object%20Reference)))

(event EventTick
  (params (DeltaSeconds :type Float%20%28single-precision%29)))

(fn ConstructionScript)