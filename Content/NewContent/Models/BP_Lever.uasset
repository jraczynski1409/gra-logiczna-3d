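; BP_Lever is an interactable lever that the player toggles with the E key while standing near it.
; Overlap events on its Box enable input for player controller 0 when a BP_PlayerCharacter enters and disable it on exit.
; Each press runs a FlipFlop that sets IsActive on or off and instantly rotates the Lever component 180 degrees forward or back.
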(event OnComponentBeginOverlap(Box)
  (params (OverlappedComponent :type Primitive%20Component%20Object%20Reference) (OtherActor :type Actor%20Object%20Reference) (OtherComp :type Primitive%20Component%20Object%20Reference) (OtherBodyIndex :type Integer) (bFromSweep :type Boolean) (SweepResult :type Hit%20Result%20Structure%20%28by%20ref%29))
  (Utilities|Casting|CastToBP_PlayerCharacter OtherActor)
  (Input|EnableInput (Game|GetPlayerController 0)))

(event OnComponentEndOverlap(Box)
  (params (OverlappedComponent :type Primitive%20Component%20Object%20Reference) (OtherActor :type Actor%20Object%20Reference) (OtherComp :type Primitive%20Component%20Object%20Reference) (OtherBodyIndex :type Integer))
  (Utilities|Casting|CastToBP_PlayerCharacter OtherActor)
  (Input|DisableInput (Game|GetPlayerController 0)))

(event Input|KeyboardEvents|E
  (params (Key :type Key%20Structure :default "None"))
  (:Pressed
    (Utilities|FlowControl|FlipFlop
      (:A
        (Variables|Default|SetisActive? true)
        (Transformation|AddRelativeRotation (Variables|Default|GetLever) "180.000000, 0, 0" false false))
      (:B
        (Variables|Default|SetisActive? false)
        (Transformation|AddRelativeRotation (Variables|Default|GetLever) "-180.000000, 0, 0" false false)))))

(fn ConstructionScript)